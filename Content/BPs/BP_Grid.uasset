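; Grid actor that spawns a configurable tile map and offers debug tools for its pathfinding.
; BeginPlay sets size, count, shape and location, and setter events respawn the map through SpawnGridMap.
; Test events pass path requests to the PathFinder with range and diagonal options.
; Visibility toggles rerun Debug, which uses looping timers to draw bounds, markers, cursor tile and neighbors, and draws the found path once.
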(event Custom|SpawnGridMap
  (Class|GridCoreGrid|SpawnGrid (Transformation|GetActorLocation) (Class|GridCoreGrid|GetGridTileSize) (Class|GridCoreGrid|GetGridTileCount) (Class|GridCoreGrid|GetGridShape))
  (CallFunction|Debug))

(event Custom|TestPath
  (bind (_isvalid _returnvalue) (Class|GridCoreGrid|GetPathFinder))
  (if _isvalid
    (Class|GridCorePathFinder|BeginCalculatePath _returnvalue (Utilities|Struct|MakeIntPoint (stale EventGridDebugTestPath StartX) (stale EventGridDebugTestPath StartY)) (Utilities|Struct|MakeIntPoint (stale EventGridDebugTestPath EnX) (stale EventGridDebugTestPath EndY)) (stale EventGridDebugTestPath Range) (Class|GridCoreGrid|GetUseDiagonal))))

(event EventGridResetGrid
  (params (TileSize :type Vector :default "0, 0, 0") (Location :type Vector :default "0, 0, 0") (TileCount :type Integer) (Shape :type EGridCoreGridShapeType%20Enum :default "None"))
  (|GridSetup TileSize Location TileCount Shape))

(event EventGridChangeTileSize
  (params (TileSize :type Vector :default "0, 0, 0"))
  (Class|GridCoreGrid|SetGridTileSize TileSize)
  (CallFunction|SpawnGridMap))

(event EventGridDebugSetDisplayNeighbors
  (params (Visibility :type Boolean))
  (Variables|Debug|SetDebugNeighbors Visibility)
  (CallFunction|Debug))

(event EventGridDebugSetUseDiagonalforNeighbors
  (params (UseDiag :type Boolean))
  (Class|GridCoreGrid|SetUseDiagonal UseDiag)
  (CallFunction|SpawnGridMap))

(event EventGridDebugClearPath
  (bind (_isvalid _returnvalue) (Class|GridCoreGrid|GetPathFinder))
  (if _isvalid
    (Class|GridCorePathFinder|ClearPath _returnvalue)))

(event EventGridDebugSetDisplayPath
  (params (Visibility :type Boolean))
  (Variables|Debug|SetDebugPath Visibility)
  (CallFunction|Debug))

(event EventGridDebugTestPath
  (params (StartX :type Integer) (StartY :type Integer) (EnX :type Integer) (EndY :type Integer) (Range :type Integer))
  (bind (_isvalid _returnvalue) (Class|GridCoreGrid|GetPathFinder))
  (if _isvalid
    (Class|GridCorePathFinder|BeginCalculatePath _returnvalue (Utilities|Struct|MakeIntPoint StartX StartY) (Utilities|Struct|MakeIntPoint EnX EndY) Range (Class|GridCoreGrid|GetUseDiagonal))))

(event EventBeginPlay
  (bind (_returnvalue _returnvalue2 _returnvalue3 _returnvalue4) (|InitWithDebugOrNot))
  (|GridSetup_2 _returnvalue _returnvalue2 _returnvalue3 _returnvalue4))

(event EventGridSetTileCount
  (params (TileCount :type Int%20Point%20Structure))
  (Class|GridCoreGrid|SetGridTileCount TileCount)
  (CallFunction|SpawnGridMap))

(event EventGridSetTileShape
  (params (Shape :type EGridCoreGridShapeType%20Enum :default "None"))
  (Class|GridCoreGrid|SetGridShape Shape)
  (CallFunction|SpawnGridMap))

(event EventGridSetUseEnvironment
  (params (UseEnvironment :type Boolean))
  (Class|GridCoreGrid|SetUseEnvironment UseEnvironment)
  (CallFunction|SpawnGridMap))

(event EventGridDebugSetDisplayBound
  (params (Visibility :type Boolean))
  (Variables|Debug|SetDisplayDebugBound Visibility)
  (CallFunction|Debug))

(event EventGridDebugSetDisplayCenter
  (params (Visibility :type Boolean))
  (Variables|Debug|SetDisplayDebugCenter Visibility)
  (CallFunction|Debug))

(event EventGridDebugSetDisplayBottomLeft
  (params (Visibility :type Boolean))
  (Variables|Debug|SetDisplayDebugBottomLeft Visibility)
  (CallFunction|Debug))

(event EventGridDebugSetDisplayMouse
  (params (Visibility :type Boolean))
  (Variables|Debug|SetDisplayDebugMouse Visibility)
  (CallFunction|Debug))

(fn ConstructionScript)

(fn DrawDebugBound
  (bind _returnvalue (Class|GridCoreGrid|GetGridTileSize))
  (bind _returnvalue_2 (/ (.x _returnvalue) 2.0))
  (if (Variables|Debug|GetDisplayDebugBound)
    (Rendering|Debug|DrawDebugSphere (Class|GridCoreGrid|GetGridCenterLocation) _returnvalue_2 6 "(R=1.000000,G=1.000000,B=0.000000,A=1.000000)" 0.5 1e+01)
    (Rendering|Debug|DrawDebugSphere (Transformation|GetActorLocation) _returnvalue_2 6 "(R=1.000000,G=0.000000,B=0.000000,A=1.000000)" 0.5 1e+01)))

(fn DrawDebugCenter
  (if (Variables|Debug|GetDisplayDebugCenter)
    (Rendering|Debug|DrawDebugSphere "0, 0, 0" 1e+02 12 "(R=1.000000,G=1.000000,B=0.000000,A=1.000000)" 0.5 1e+01)))

(fn DrawDebugBottomLeft
  (if (Variables|Debug|GetDisplayDebugBottomLeft)
    (Rendering|Debug|DrawDebugSphere "0, 0, 0" 1e+02 6 "(R=1.000000,G=1.000000,B=0.000000,A=1.000000)" 0.5 1e+01)))

(fn DrawDebugMouse
  (if (Variables|Debug|GetDisplayDebugMouse)
    (bind _returnvalue (Class|GridCoreGrid|GetCursorLocation))
    (Rendering|Debug|DrawDebugSphere _returnvalue 7.0 6 "(R=1.000000,G=1.000000,B=0.000000,A=1.000000)" 0.1 2.0)
    (bind _returnvalue_2 (Class|GridCoreGrid|GetIndexwithLocation _returnvalue))
    (if (.ReturnValue (Class|GridCoreGrid|GetTilePropertiesbyIndex _returnvalue_2))
      (Rendering|Debug|DrawDebugSphere (.Location (Class|GridCoreGrid|GetTilePropertiesbyIndex _returnvalue_2)) 1e+01 6 "(R=1.000000,G=0.000000,B=0.000000,A=1.000000)" (Utilities|Time|GetWorldDeltaSeconds) 3.0))))

(fn DrawDebugNeighbors
  (if (Variables|Debug|GetDebugNeighbors)
    (bind _returnvalue (Class|GridCoreGrid|GetCursorLocation))
    (bind _returnvalue_2 (Class|GridCoreGrid|GetIndexwithLocation _returnvalue))
    (if (.ReturnValue (Class|GridCoreGrid|GetTilePropertiesbyIndex _returnvalue_2))
      (for _array_element (.Neighbors (Class|GridCoreGrid|GetTilePropertiesbyIndex _returnvalue_2))
        (if (.ReturnValue (Class|GridCoreGrid|GetTilePropertiesbyIndex _array_element))
          (Rendering|Debug|DrawDebugSphere (.Location (Class|GridCoreGrid|GetTilePropertiesbyIndex _array_element)) 15.0 12 "(R=0.296541,G=0.000000,B=1.000000,A=1.000000)" (Utilities|Time|GetWorldDeltaSeconds) 3.0)))
      (Development|PrintString (Utilities|String|ToString(Integer) (Utilities|Array|Length (.Neighbors (Class|GridCoreGrid|GetTilePropertiesbyIndex _returnvalue_2))))))))

(fn Debug
  (Utilities|FlowControl|Sequence
    (:then_0
      (Utilities|Time|SetTimerbyEvent (EventDispatchers|CreateEvent :!event DrawDebugBound) 0.5 (Variables|Debug|GetDisplayDebugBound)))
    (:then_1
      (Utilities|Time|SetTimerbyEvent (EventDispatchers|CreateEvent :!event DrawDebugCenter) 0.5 (Variables|Debug|GetDisplayDebugCenter)))
    (:then_2
      (Utilities|Time|SetTimerbyEvent (EventDispatchers|CreateEvent :!event DrawDebugBottomLeft) 0.5 (Variables|Debug|GetDisplayDebugBottomLeft)))
    (:then_3
      (Utilities|Time|SetTimerbyEvent (EventDispatchers|CreateEvent :!event DrawDebugMouse) (Utilities|Time|GetWorldDeltaSeconds) (Variables|Debug|GetDisplayDebugMouse)))
    (:then_4
      (Utilities|Time|SetTimerbyEvent (EventDispatchers|CreateEvent :!event DrawDebugNeighbors) (Utilities|Time|GetWorldDeltaSeconds) (Variables|Debug|GetDebugNeighbors)))
    (:then_5
      (CallFunction|DrawDebugPath))))

(fn DrawDebugPath
  (if (Variables|Debug|GetDebugPath)
    (bind (_isvalid _returnvalue) (Class|GridCoreGrid|GetPathFinder))
    (if _isvalid
      (bind _returnvalue_2 (Class|GridCorePathFinder|GetPathFound _returnvalue))
      (for _array_element _returnvalue_2
        (if (.ReturnValue (Class|GridCoreGrid|GetTilePropertiesbyIndex _array_element))
          (Rendering|Debug|DrawDebugSphere (.Location (Class|GridCoreGrid|GetTilePropertiesbyIndex _array_element)) 14.0 12 "(R=1.000000,G=1.000000,B=1.000000,A=1.000000)" 1e+01 14.0))))))