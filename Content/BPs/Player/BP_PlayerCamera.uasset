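; Player camera Blueprint that rotates around its spring arm in yaw steps and creates the game UI widget.
; On BeginPlay it eases the camera toward an Arrow component with a pitch offset, passes the widget to the game state via interface and caches the arm rotation.
; ChangeCameraRotation adds a yaw offset and lerps the spring arm there on a timeline, with CanTurn blocking overlapping turns.
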(event Custom|OnCameraLookAt
  (|MakeCameraLookAt))

(event EventBeginPlay
  (Utilities|FlowControl|Sequence
    (:then_0
      (|MakeCameraLookAt))
    (:then_1
      (|MakeWidget))
    (:then_2
      (|GetCamRot))))

(event EventChangeCameraRotation
  (params (AddingRotation :type Rotator :default "0, 0, 0"))
  (if (Variables|Default|GetCanTurn)
    (Variables|Default|SetCanTurn false)
    (bind _newrotation (CallFunction|CalculateNexRotation AddingRotation (Variables|Default|GetCurrentCameraRotation)))
    (bind _alpha (Timeline|Timeline_0 PlayFromStart)
      (:Update
        (Transformation|SetWorldRotation (Variables|Default|GetSpringArm) (Math|Rotator|Lerp(Rotator) (Variables|Default|GetCurrentCameraRotation) _newrotation _alpha true) false false))
      (:Finished
        (Variables|Default|SetCurrentCameraRotation _newrotation)
        (Variables|Default|SetCanTurn true)))))

(fn ConstructionScript)

(fn CalculateNexRotation
  (params (Offset :type Rotator) (CurrentRotation :type Rotator))
  (return (Math|Rotator|MakeRotator (.roll CurrentRotation) (.pitch CurrentRotation) (Class|KismetMathLibrary|ClampAxis (+ (.yaw CurrentRotation) (.yaw Offset))))))