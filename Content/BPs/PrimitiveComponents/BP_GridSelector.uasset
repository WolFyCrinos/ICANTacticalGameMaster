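; BP_GridSelector is a component that shows a visual effect as a grid selection marker.
; On BeginPlay it spawns the SelectorFX system at its world transform, stores it as FX and hides it.
; SetGridSelectorActive toggles that effect's visibility.
; The effect is spawned at a location rather than attached, and uses auto-release pooling although its reference is kept.
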(event EventBeginPlay
  (bind _self self)
  (bind _returnvalue (Transformation|GetWorldTransform _self))
  (bind _returnvalue_2 (Niagara|SpawnSystematLocation (Variables|Default|GetSelectorFX) (.location _returnvalue) (.rotation _returnvalue) (.scale _returnvalue) true true "AutoRelease"))
  (bind _output_get (Variables|Default|SetFX _returnvalue_2))
  (Rendering|SetVisibility _output_get false false))

(fn SetGridSelectorActive
  (params (bIsActive :type Boolean))
  (bind _fx (Variables|Default|GetFX))
  (if bIsActive
    (Rendering|SetVisibility _fx true false)
    (else
      (Rendering|SetVisibility _fx false false))))