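; BP_Cube is a map element cube that plays a dissolve effect and shows a grid selector under the cursor.
; On BeginPlay, a timeline drives the Dissolve and DissolveEmissive scalars in the MP_MapElement parameter collection, so the values are shared rather than set per cube.
; Cursor begin and end over events on the Cube component toggle BPGridSelector, only when the cube is walkable.
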(event OnBeginCursorOver(Cube)
  (params (TouchedComponent :type Primitive%20Component%20Object%20Reference))
  (if (Variables|Default|GetbIsWalkable)
    (Default|SetGridSelectorActive (Variables|Default|GetBP_GridSelector) true)))

(event OnEndCursorOver(Cube)
  (params (TouchedComponent :type Primitive%20Component%20Object%20Reference))
  (if (Variables|Default|GetbIsWalkable)
    (Default|SetGridSelectorActive (Variables|Default|GetBP_GridSelector) false)))

(event EventBeginPlay
  (Utilities|FlowControl|Sequence
    (:then_0
      (bind (_direction _alpha _emissivedissolve) (Timeline|Dissolve PlayFromStart)
        (:Update
          (Rendering|Material|SetScalarParameterValue "/Game/Materials/Parameters/MP_MapElement.MP_MapElement" "Dissolve" _alpha :!class /Script/Engine.KismetMaterialLibrary)
          (Rendering|Material|SetScalarParameterValue "/Game/Materials/Parameters/MP_MapElement.MP_MapElement" "DissolveEmissive" _emissivedissolve :!class /Script/Engine.KismetMaterialLibrary))))))

(fn ConstructionScript)