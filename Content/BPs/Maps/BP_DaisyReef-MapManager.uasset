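; Map manager for the DaisyReef map that, as shown here, runs a pathfinding test on BeginPlay.
; It asks DaisyRefPathFinder for a ranged path between two hardcoded entries in FloorMapElementsSpawned.
; For each element in the returned path it prints the F score and draws a persistent debug line trace to its previous element at a fixed height.
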(event Custom|PathFindTest
  (bind _floormapelementsspawned (Variables|Default|GetFloorMapElementsSpawned))
  (Class|DaisyRefPathFinder|FindPath (Variables|Default|GetDaisyRefPathFinder) (Utilities|Array|Get(acopy) _floormapelementsspawned 10) (Utilities|Array|Get(acopy) _floormapelementsspawned 152) 5)
  (bind _returnvalue (Class|DaisyRefPathFinder|GetPath (Variables|Default|GetDaisyRefPathFinder)))
  (for _array_element _returnvalue
    (bind _returnvalue_2 (Class|DaisyReefMapElement|GetF _array_element))
    (Development|PrintString (Utilities|String|ToString(Integer) _returnvalue_2))
    (bind _returnvalue_3 (Class|DaisyReefMapElement|GetPrevious _array_element))
    (Collision|LineTraceByChannel (Math|Vector|MakeVector (.x (Transformation|GetActorLocation _array_element)) (.y (Transformation|GetActorLocation _array_element)) 2e+02) (Math|Vector|MakeVector (.x (Transformation|GetActorLocation _returnvalue_3)) (.y (Transformation|GetActorLocation _returnvalue_3)) 2e+02) "TraceTypeQuery1" false 0 "Persistent")))

(event EventBeginPlay
  (bind _floormapelementsspawned (Variables|Default|GetFloorMapElementsSpawned))
  (Class|DaisyRefPathFinder|FindPath (Variables|Default|GetDaisyRefPathFinder) (Utilities|Array|Get(acopy) _floormapelementsspawned 10) (Utilities|Array|Get(acopy) _floormapelementsspawned 152) 5)
  (bind _returnvalue (Class|DaisyRefPathFinder|GetPath (Variables|Default|GetDaisyRefPathFinder)))
  (for _array_element _returnvalue
    (bind _returnvalue_2 (Class|DaisyReefMapElement|GetF _array_element))
    (Development|PrintString (Utilities|String|ToString(Integer) _returnvalue_2))
    (bind _returnvalue_3 (Class|DaisyReefMapElement|GetPrevious _array_element))
    (Collision|LineTraceByChannel (Math|Vector|MakeVector (.x (Transformation|GetActorLocation _array_element)) (.y (Transformation|GetActorLocation _array_element)) 2e+02) (Math|Vector|MakeVector (.x (Transformation|GetActorLocation _returnvalue_3)) (.y (Transformation|GetActorLocation _returnvalue_3)) 2e+02) "TraceTypeQuery1" false 0 "Persistent")))

(fn ConstructionScript)